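; BP_Attributes is a Blueprint that tracks the health of its owner.
; On BeginPlay it sets current health to the maximum.
; ReduceHealth subtracts damage, clamps the result between zero and the maximum, and returns the new health along with a flag for death when it reaches zero.
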(event `self.ReceiveBeginPlay`
  (set `self.CurrentHealth` (`self.Maxhealth`)))

(fn `ReduceHealth`
  (params (DamageAmount :type "Float (double-precision)"))
  (returns (UpdateHealth :type "Float (double-precision)") (isDied :type Boolean))
  (bind _output_get (set `self.CurrentHealth` (`KismetMathLibrary.FClamp` (- (`self.CurrentHealth`) DamageAmount) 0.0 (`self.Maxhealth`))))
  (return _output_get (== (`self.CurrentHealth`) 0.0)))