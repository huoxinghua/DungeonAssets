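; BP_BaseTrap is a trap actor that damages and launches the first-person player character on overlap with its hit volume.
; It passes its damage amount, type and itself to TakeDamage, then launches along GetAwayDirection scaled by LaunchPower, overriding XY velocity only.
; Despite its name, GetAwayDirection points from player to trap.
; Traps tagged "Noneammo" destroy themselves after the hit.
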(event `self.HitDetectVolume.OnComponentBeginOverlap`
  (params (OverlappedComponent :type "PrimitiveComponent Object Reference") (OtherActor :type "Actor Object Reference") (OtherComp :type "PrimitiveComponent Object Reference") (OtherBodyIndex :type Integer) (bFromSweep :type Boolean) (SweepResult :type "HitResult Structure (by ref)"))
  (bind _asbp_first_person_character (cast `/Game/FirstPerson/Blueprints/BP_FirstPersonCharacter` OtherActor))
  (`/Game/FirstPerson/Blueprints/BP_FirstPersonCharacter.TakeDamage` _asbp_first_person_character (make `/Game/MyBP/Struct_HitInfo` (`self.DamageAmount`) (`self.DamageType`) self))
  (`Character.LaunchCharacter` _asbp_first_person_character (* (`self.GetAwayDirection` _asbp_first_person_character) (`self.LaunchPower`)) true false)
  (if (`self.ActorHasTag` "Noneammo")
    (`self.K2_DestroyActor`)
    (`KismetSystemLibrary.PrintString` "Hello")))

(fn `GetAwayDirection`
  (params (self2 :type "Actor Object Reference"))
  (returns (ReturnValue :type "Vector Structure"))
  (return (`KismetMathLibrary.Normal` (- (`self.K2_GetActorLocation`) (`self.K2_GetActorLocation` self2)))))

(fn `UserConstructionScript`)