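; BP_MovingTrap is a trap that continuously moves its TrapMesh back and forth along a line toward a destination.
; Tick sets the mesh's relative location by lerping StartPosition to DestinationPosition with a sine of time since creation, scaled by Speed and Dampening.
; The absolute sine is remapped to 0.5–1, so motion covers only the destination half of the path.
; BeginPlay starts a looping timer on an empty event.
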(event `self.ReceiveBeginPlay`
  (`KismetSystemLibrary.K2_SetTimerDelegate` (delegate `CustomEvent`) 1.0 true))

(event `CustomEvent`)

(event `self.ReceiveTick`
  (params (DeltaSeconds :type "Float (single-precision)"))
  (`SceneComponent.K2_SetRelativeLocation` (`self.TrapMesh`) (`KismetMathLibrary.VLerp` (`self.StartPosition`) (`self.DestinationPosition`) (/ (+ (`KismetMathLibrary.Abs` (`KismetMathLibrary.Sin` (* (/ (`self.GetGameTimeSinceCreation`) (`self.Dampening`)) (`self.speed`)))) 1.0) 2.0)) false false))

(fn `UserConstructionScript`
  (`parent.UserConstructionScript`))