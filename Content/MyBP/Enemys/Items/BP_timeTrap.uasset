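; BP_timeTrap is a timed trap that alternates between hidden and active states, starting deactivated on BeginPlay.
; DeactivateTrap and ActivateTrap toggle the mesh visibility and the HitDetectVolume collision, then each sets a timer event using the Deactivated or Activated duration, apparently to flip states.
; The mesh itself never collides, and no hit response is defined here.
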(event `self.ReceiveBeginPlay`
  (`PrimitiveComponent.SetCollisionEnabled` (`self.TrapMesh`) "NoCollision")
  (`self.DeactivateTrap`))

(fn `Activate Trap`
  (`SceneComponent.SetVisibility` (`self.TrapMesh`) true false)
  (`PrimitiveComponent.SetCollisionEnabled` (`self.HitDetectVolume`) "QueryAndPhysics")
  (`KismetSystemLibrary.K2_SetTimerDelegate` (`|CreateDelegate` :!event `DeactivateTrap`) (`self.Activated`)))

(fn `DeactivateTrap`
  (`SceneComponent.SetVisibility` (`self.TrapMesh`) false false)
  (`PrimitiveComponent.SetCollisionEnabled` (`self.HitDetectVolume`) "NoCollision")
  (`KismetSystemLibrary.K2_SetTimerDelegate` (`|CreateDelegate` :!event `Activate Trap`) (`self.Deactivated`)))

(fn `UserConstructionScript`
  (`parent.UserConstructionScript`))