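; Item spawner actor that periodically places a random trap from its TrapToSpawn class array at its own location and rotation.
; A looping timer started on BeginPlay retries every few seconds, spawning only when the tracked CurrentItem is no longer valid, so one spawned actor exists at a time.
; Otherwise it just prints a message; the ItemToSpawn variable is unused.
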(event `self.ReceiveBeginPlay`
  (`KismetSystemLibrary.K2_SetTimerDelegate` (delegate `RespawnItem`) 5.0 true))

(event `RespawnItem`
  (`self.AttemptToSpawn`))

(fn `AttemptToSpawn`
  (`/Engine/EditorBlueprintResources/StandardMacros.IsValid` (`self.CurrentItem`)
    (:`Is Valid`
      (`KismetSystemLibrary.PrintString` "Items already spawned"))
    (:`Is Not Valid`
      (`self.SpawnItem`))))

(fn `SpawnItem`
  (bind _returnvalue (`|SpawnActorFromClass` (`|GetArrayItem` (`self.TrapToSpawn`) (`KismetMathLibrary.RandomIntegerInRange` 0 (- (`KismetArrayLibrary.Array_Length` (`self.TrapToSpawn`)) 1))) (`KismetMathLibrary.MakeTransform` (`self.K2_GetActorLocation`) (`self.K2_GetActorRotation`)) "AdjustIfPossibleButAlwaysSpawn" "MultiplyWithRoot" null null))
  (set `self.CurrentItem` _returnvalue))

(fn `UserConstructionScript`)