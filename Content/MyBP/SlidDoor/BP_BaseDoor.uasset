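; BP_BaseDoor is a door actor driven by overlaps on its HitBox.
; A third-person character entering plays the OPENDOOR timeline, while the exit handler reverses it only for a first-person character.
; Each timeline update prints WelcomeText and sets the relative Y of the Left and Right parts to the same scaled curve value, so both move in the same local direction.
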(event `self.HitBox.OnComponentBeginOverlap`
  (params (OverlappedComponent :type "PrimitiveComponent Object Reference") (OtherActor :type "Actor Object Reference") (OtherComp :type "PrimitiveComponent Object Reference") (OtherBodyIndex :type Integer) (bFromSweep :type Boolean) (SweepResult :type "HitResult Structure (by ref)"))
  (cast `/Game/ThirdPerson/Blueprints/BP_ThirdPersonCharacter` OtherActor)
  (bind (_direction _opendoor) (`Timeline|OPENDOOR` :!label _label)
    (:`Update`
      (`KismetSystemLibrary.PrintText` (`self.WelcomeText`))
      (`SceneComponent.K2_SetRelativeLocation` (`self.Left`) (`KismetMathLibrary.MakeVector` 0.0 (* _opendoor 100.0)) false false)
      (`SceneComponent.K2_SetRelativeLocation` (`self.Right`) (`KismetMathLibrary.MakeVector` 0.0 (* _opendoor 100.0)) false false))))

(event `self.HitBox.OnComponentEndOverlap`
  (params (OverlappedComponent :type "PrimitiveComponent Object Reference") (OtherActor :type "Actor Object Reference") (OtherComp :type "PrimitiveComponent Object Reference") (OtherBodyIndex :type Integer))
  (cast `/Game/FirstPerson/Blueprints/BP_FirstPersonCharacter` OtherActor)
  (goto _label :!via `Reverse`))

(fn `UserConstructionScript`)