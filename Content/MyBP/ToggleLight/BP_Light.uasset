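; BP_Light is a proximity-triggered light that turns on when a Character enters its box collision and off shortly after one leaves.
; On begin overlap it shows the PointLight and gives it a random color converted from a random unit vector.
; On end overlap it waits two seconds, then hides the light without checking whether a Character has re-entered.
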(event `self.BoxCollision.OnComponentBeginOverlap`
  (params (OverlappedComponent :type "PrimitiveComponent Object Reference") (OtherActor :type "Actor Object Reference") (OtherComp :type "PrimitiveComponent Object Reference") (OtherBodyIndex :type Integer) (bFromSweep :type Boolean) (SweepResult :type "HitResult Structure (by ref)"))
  (bind _pointlight (`self.PointLight`))
  (cast `Character` OtherActor)
  (`SceneComponent.SetVisibility` _pointlight true false)
  (`LightComponent.SetLightColor` _pointlight (`KismetMathLibrary.Conv_VectorToLinearColor` (`KismetMathLibrary.RandomUnitVector`)) true))

(event `self.BoxCollision.OnComponentEndOverlap`
  (params (OverlappedComponent :type "PrimitiveComponent Object Reference") (OtherActor :type "Actor Object Reference") (OtherComp :type "PrimitiveComponent Object Reference") (OtherBodyIndex :type Integer))
  (cast `Character` OtherActor)
  (`KismetSystemLibrary.Delay` 2.0)
  (`SceneComponent.SetVisibility` (`self.PointLight`) false false))

(fn `UserConstructionScript`)